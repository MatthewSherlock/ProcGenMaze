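; AI controller for enemies that runs the BT_Enemy behavior tree on possess and feeds it player perception.
; Sensing an actor tagged Player cancels the lose-sight timer and writes the HasLineOfSight and Player blackboard keys.
; Any other perception update starts a one-shot timer of LineOfSightTimer length, which clears both keys on expiry, giving a grace period before the enemy loses the player.
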(event `self.ReceivePossess`
  (params (PossessedPawn :type "Pawn Object Reference"))
  (`self.RunBehaviorTree` "/Game/AI/BT_Enemy.BT_Enemy"))

(event `self.AIPerception.OnTargetPerceptionUpdated`
  (params (Actor :type "Actor Object Reference") (Stimulus :type "AIStimulus Structure"))
  (bind _returnvalue (`AIBlueprintHelperLibrary.GetBlackboard` null))
  (if (and (`self.ActorHasTag` Actor "Player") (`.bSuccessfullySensed` (break `AIStimulus` Stimulus)))
    (`KismetSystemLibrary.K2_ClearAndInvalidateTimerHandle` (`self.EnemyTimer`))
    (`BlackboardComponent.SetValueAsBool` _returnvalue (`self.HasLineOfSight`) true)
    (`BlackboardComponent.SetValueAsObject` _returnvalue (`self.Player`) Actor)
    (else
      (bind _returnvalue_2 (`KismetSystemLibrary.K2_SetTimerDelegate` (delegate `StartEnemyTimer`) (`self.LineOfSightTimer`)))
      (set `self.EnemyTimer` _returnvalue_2))))

(event `StartEnemyTimer`
  (bind _returnvalue (`AIBlueprintHelperLibrary.GetBlackboard` null))
  (`BlackboardComponent.SetValueAsBool` _returnvalue (`self.HasLineOfSight`) false)
  (`BlackboardComponent.SetValueAsObject` _returnvalue (`self.Player`) null))

(fn `UserConstructionScript`)