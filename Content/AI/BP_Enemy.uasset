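; BP_Enemy is an AI enemy that freezes while seen by the player and can grab the player on contact.
; Capsule overlap with the first-person character sets the IsGrabbing blackboard key if CanGrab is true, and prints a debug string.
; Unless grabbing, each SeenbyPlayer call disables movement and restarts a short retriggerable delay, so nav walking resumes only once the calls stop.
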(event `self.CapsuleComponent.OnComponentBeginOverlap`
  (params (OverlappedComponent :type "PrimitiveComponent Object Reference") (OtherActor :type "Actor Object Reference") (OtherComp :type "PrimitiveComponent Object Reference") (OtherBodyIndex :type Integer) (bFromSweep :type Boolean) (SweepResult :type "HitResult Structure (by ref)"))
  (bind _returnvalue (`AIBlueprintHelperLibrary.GetBlackboard` null))
  (cast `/Game/FirstPersonCPP/Blueprints/FirstPersonCharacter` OtherActor)
  (if (`BlackboardComponent.GetValueAsBool` _returnvalue (`self.CanGrab`))
    (`BlackboardComponent.SetValueAsBool` _returnvalue (`self.isGrabbing`) true)
    (`KismetSystemLibrary.PrintString` "Hello")))

(event `self.SeenByPlayer`
  (bind _charactermovement (`self.CharacterMovement`))
  (if (not (`BlackboardComponent.GetValueAsBool` (`AIBlueprintHelperLibrary.GetBlackboard` null) (`self.isGrabbing`)))
    (`|ExecutionSequence`
      (:`then_0`
        (`CharacterMovementComponent.DisableMovement` _charactermovement))
      (:`then_1`
        (`KismetSystemLibrary.RetriggerableDelay` 0.4)
        (`CharacterMovementComponent.SetMovementMode` _charactermovement "MOVE_NavWalking" 0)))))

(fn `UserConstructionScript`)